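; Main base building that acts as a power source, emitting a recurring pulse to nearby power nodes.
; BeginPlay starts a looping timer that fires EmitPowerPulse every PulseInterval.
; Each pulse calls ReceivePowerPulse on every BP_PowerNode overlapping PowerRange.
; The IsPusing flag is set at pulse start and cleared by a short Delay inside the loop, so it resets only when nodes are found.
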(event `self.ReceiveBeginPlay`
  (`KismetSystemLibrary.K2_SetTimer` null "EmitPowerPulse" (`self.PulseInterval`) true))

(event `EmitPowerPulse`
  (set `self.bIsPusing` true)
  (for _array_element (`PrimitiveComponent.GetOverlappingActors` (`self.PowerRange`) "/Game/Blueprints/Buildings/BP_PowerNode.BP_PowerNode_C")
    (bind _asbp_power_node (cast `/Game/Blueprints/Buildings/BP_PowerNode` _array_element))
    (`/Game/Blueprints/Buildings/BP_PowerNode.ReceivePowerPulse` _asbp_power_node null)
    (`KismetSystemLibrary.Delay` (* (`self.PulseInterval`) 0.1))
    (set `self.bIsPusing` false)))

(fn `UserConstructionScript`)